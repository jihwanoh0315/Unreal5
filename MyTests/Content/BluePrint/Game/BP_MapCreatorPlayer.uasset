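; Map creator player that views the level through a tagged TopDownCam camera and drags objects with the mouse.
; G toggles grab mode and the cursor, and caches actors tagged Block.
; In grab mode, left click traces from the cursor to grab a Movable component until release.
; Tick moves simulating components via PhysicsHandle at the original hit distance, and snaps others to a cursor trace that ignores the Blocks, with debug output.
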(event `Key|G`
  (params (Key :type "Key Structure"))
  (bind _returnvalue (`GameplayStatics.GetPlayerController` 0))
  (:`Pressed`
    (bind _outactors (`GameplayStatics.GetAllActorsWithTag` "Block"))
    (set `self.Blocks` _outactors)
    (set `self.GrabMode` (not (`self.GrabMode`)))
    (set `PlayerController.bShowMouseCursor` (not (`PlayerController.bShowMouseCursor` _returnvalue)) _returnvalue)))

(event `self.ReceiveBeginPlay`
  (bind _outactors (`GameplayStatics.GetAllActorsOfClassWithTag` "/Script/Engine.CameraActor" "TopDownCam"))
  (for _array_element _outactors
    (`PlayerController.SetViewTargetWithBlend` (`GameplayStatics.GetPlayerController` 0) _array_element 0.0 "VTBlend_Linear" 0.0 false)))

(event `Key|LeftMouseButton`
  (params (Key :type "Key Structure"))
  (bind _grabmode (`self.GrabMode`))
  (bind (_worldlocation _worlddirection) (`PlayerController.DeprojectMousePositionToWorld` (`GameplayStatics.GetPlayerController` 0)))
  (:`Pressed`
    (if _grabmode
      (bind (_outhit _returnvalue) (`KismetSystemLibrary.LineTraceSingle` :`Start` _worldlocation :`End` (+ _worldlocation (* _worlddirection 10000.0)) :`TraceChannel` "TraceTypeQuery1" :`bTraceComplex` true :`DrawDebugType` "ForDuration"))
      (if _returnvalue
        (if (`|EnumEquality` (`SceneComponent.Mobility` (`.HitComponent` (`GameplayStatics.BreakHitResult` _outhit))) (enumliteral `EComponentMobility` "Movable"))
          (bind (_bblockinghit _binitialoverlap _time _distance _location _impactpoint _normal _impactnormal _physmat _hitactor _hitcomponent) (`GameplayStatics.BreakHitResult` _outhit))
          (set `self.OriginalDistance` _distance)
          (bind _output_get (set `self.GrabbedComponent` _hitcomponent))
          (if (`SceneComponent.IsSimulatingPhysics` _output_get "None")
            (`PhysicsHandleComponent.GrabComponentAtLocation` (`self.PhysicsHandle`) (`self.GrabbedComponent`) "None" (`.Location` (`GameplayStatics.BreakHitResult` _outhit))))))))
  (:`Released`
    (if _grabmode
      (set `self.GrabbedComponent` null)
      (`PhysicsHandleComponent.ReleaseComponent` (`self.PhysicsHandle`)))))

(event `self.ReceiveTick`
  (params (DeltaSeconds :type "Float (single-precision)"))
  (bind _grabbedcomponent (`self.GrabbedComponent`))
  (bind (_worldlocation _worlddirection) (`PlayerController.DeprojectMousePositionToWorld` (`GameplayStatics.GetPlayerController` 0)))
  (bind (_worldlocation_2 _worlddirection_2) (`PlayerController.DeprojectMousePositionToWorld` (`GameplayStatics.GetPlayerController` 0)))
  (`/Engine/EditorBlueprintResources/StandardMacros.IsValid` _grabbedcomponent
    (:`Is Valid`
      (`KismetSystemLibrary.PrintString` (`KismetSystemLibrary.GetDisplayName` _grabbedcomponent) true true (struct :`G` 0.66 :`B` 1.0 :`A` 1.0) 0.0)
      (if (`self.GrabMode`)
        (if (`SceneComponent.IsSimulatingPhysics` _grabbedcomponent "None")
          (`PhysicsHandleComponent.SetTargetLocation` (`self.PhysicsHandle`) (+ _worldlocation_2 (* _worlddirection_2 (`self.OriginalDistance`))))
          (else
            (bind (_outhit _returnvalue) (`KismetSystemLibrary.LineTraceSingle` _worldlocation (+ _worldlocation (* _worlddirection 10000.0)) "TraceTypeQuery1" true (`self.Blocks`) "ForDuration" true (struct :`R` 0.045644 :`G` 0.102498 :`B` 1.0 :`A` 1.0)))
            (if _returnvalue
              (bind (_bblockinghit _binitialoverlap _time _distance _location _impactpoint _normal _impactnormal _physmat _hitactor) (`GameplayStatics.BreakHitResult` _outhit))
              (`SceneComponent.K2_SetWorldLocation` (`self.GrabbedComponent`) _impactpoint false false)
              (`KismetSystemLibrary.PrintString` (`KismetStringLibrary.Conv_VectorToString` (`SceneComponent.K2_GetComponentScale` (`Actor.RootComponent` _hitactor)))))))))))

(fn `UserConstructionScript`)