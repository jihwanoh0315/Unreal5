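; BP_EditorPlayer handles placing notes in a note editor.
; SpawnNote moves the mouse to the screen origin, spawns a BP_EditorNote at the world origin and holds it as the grabbed note, flagged as created.
; CheckOverlapAndReturn compares the grabbed note's sprite position against notes sharing its tags, returning it to its grab location on an exact overlap, with the selection marker offset slightly in Y.
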(fn `CheckOverlapAndReturn`
  (bind _grabbednote (`self.GrabbedNote`))
  (bind _grabbedlocation (`self.GrabbedLocation`))
  (bind (_x _y _z) (`KismetMathLibrary.BreakVector3f` _grabbedlocation))
  (for _array_element (`Actor.Tags` (`self.GrabbedNote`))
    (bind _outactors (`GameplayStatics.GetAllActorsOfClassWithTag` "/Game/BluePrints/Game/BP_EditorNote.BP_EditorNote_C" _array_element))
    (for _array_element_2 _outactors
      (if (!= _array_element_2 _grabbednote)
        (if (== (`SceneComponent.K2_GetComponentLocation` (`/Game/BluePrints/Game/BP_EditorNote.PaperSprite` _array_element_2)) (`SceneComponent.K2_GetComponentLocation` (`/Game/BluePrints/Game/BP_EditorNote.PaperSprite` _grabbednote)))
          (`self.K2_SetActorLocation` _grabbednote _grabbedlocation false false)
          (`self.K2_SetActorLocation` (`self.NoteSelected`) (`KismetMathLibrary.MakeVector` _x (+ _y 1.0) _z) false false)
          (break))))))

(fn `SpawnNote`
  (`PlayerController.SetMouseLocation` (`GameplayStatics.GetPlayerController` 0) 0 0)
  (bind _returnvalue (`|SpawnActorFromClass` "/Game/BluePrints/Game/BP_EditorNote.BP_EditorNote_C" (`KismetMathLibrary.MakeTransform` (0.0 0.0 0.0)) "Undefined" "OverrideRootScale" null null))
  (set `self.GrabbedNote` _returnvalue)
  (set `self.isCreated` true))

(fn `UserConstructionScript`)